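; BP_InkyTarget is the target actor for the ghost Inky in a Pac-Man game, marking a point derived from Pac-Man and Blinky.
; It caches the Pac-Man character on BeginPlay, then moves itself to the computed target each Tick and draws a cyan debug box there.
; GetTargetPosition projects a Distance ahead along Pac-Man's current direction, then extends past that point, away from Blinky, by half the Blinky-to-point vector.
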(event `self.ReceiveBeginPlay`
  (bind _returnvalue (`GameplayStatics.GetActorOfClass` "/Game/Blueprints/BP_PacManCharacter.BP_PacManCharacter_C"))
  (set `self.PlayerActor` _returnvalue))

(event `self.ReceiveTick`
  (params (DeltaSeconds :type "Float (single-precision)"))
  (bind _targetlocation (`self.GetTargetPosition`))
  (`self.K2_SetActorLocation` _targetlocation)
  (`KismetSystemLibrary.DrawDebugBox` _targetlocation (3.0 3.0 3.0) (struct :`G` 1.0 :`B` 1.0 :`A` 1.0)))

(fn `GetTargetPosition`
  (returns (TargetLocation :type "Vector Structure"))
  (locals (OffsetPosition :type "Vector Structure"))
  (bind _playeractor (`self.PlayerActor`))
  (bind (_x _y) (`KismetMathLibrary.BreakVector2D` (`PacMan_Character.CurrentDirection` _playeractor)))
  (set `local.OffsetPosition` (+ (`self.K2_GetActorLocation` _playeractor) (* (`KismetMathLibrary.MakeVector` _x _y) (`self.Distance`))))
  (return (+ (`KismetMathLibrary.NegateVector` (/ (- (`self.K2_GetActorLocation` (`self.BlinkyActor`)) (`local.OffsetPosition`)) 2)) (`local.OffsetPosition`))))

(fn `UserConstructionScript`)