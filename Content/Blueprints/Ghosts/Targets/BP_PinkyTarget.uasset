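; BP_PinkyTarget is the target point actor for the ghost Pinky in a Pac-Man game, kept ahead of the player.
; On BeginPlay it finds and stores the BP_PacManCharacter.
; Each Tick it moves itself to the player's location offset by the player's CurrentDirection, flattened to Z=0 and scaled by Distance.
; It also draws a small pink debug box at that point every frame.
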(event `self.ReceiveBeginPlay`
  (bind _returnvalue (`GameplayStatics.GetActorOfClass` "/Game/Blueprints/BP_PacManCharacter.BP_PacManCharacter_C"))
  (set `self.PlayerActor` _returnvalue))

(event `self.ReceiveTick`
  (params (DeltaSeconds :type "Float (single-precision)"))
  (bind _playeractor (`self.PlayerActor`))
  (bind (_x _y) (`KismetMathLibrary.BreakVector2D` (`PacMan_Character.CurrentDirection` _playeractor)))
  (bind _returnvalue (+ (`self.K2_GetActorLocation` _playeractor) (* (`KismetMathLibrary.MakeVector` _x _y) (`self.Distance`))))
  (`self.K2_SetActorLocation` _returnvalue)
  (`KismetSystemLibrary.DrawDebugBox` _returnvalue (3.0 3.0 3.0) (struct :`R` 1.0 :`G` 0.265021 :`B` 0.676057 :`A` 1.0)))

(fn `UserConstructionScript`)